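; BP_Jail is an interactable door, apparently for a jail, that swings by setting the yaw of its static mesh.
; On Interaction, a locked door plays a separate Timeline from the start, while an unlocked one toggles IsClosed and plays or reverses the RotationDoor timeline.
; Both timelines scale their output by a negated RotationAngle.
; Construction-script logic for presetting the open or closed pose is disconnected.
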(event EventBeginPlay)

(event Collision|EventActorBeginOverlap
  (params (OtherActor :type Actor%20Object%20Reference)))

(event EventTick
  (params (DeltaSeconds :type Float%20%28single-precision%29)))

(event EventInteraction
  (if (Variables|Default|GetIsLocked)
    ;[1 0.7317 0.237] Smooth_Open
    (bind _rotationvalue (Timeline|Timeline PlayFromStart)
      (:Update
        (Transformation|SetRelativeRotation (Variables|Default|GetDoor_3_StaticMeshComponent0) (Math|Rotator|MakeRotator 0.0 0.0 (* _rotationvalue (Variables|Default|GetRotationAngle) -1.0)) false false)))
    (else
      ;[0.07409 0.7375 1] Open_Rotation
      (if (Variables|Default|GetIsClosed)
        (Variables|Default|SetIsClosed false)
        (bind _rotationvalue_2 (Timeline|RotationDoor Play)
          (:Update
            (Transformation|SetRelativeRotation (Variables|Default|GetDoor_3_StaticMeshComponent0) (Math|Rotator|MakeRotator 0.0 0.0 (* _rotationvalue_2 (Variables|Default|GetRotationAngle) -1.0)) false false)))
        (else
          (Variables|Default|SetIsClosed true)
          (Timeline|RotationDoor Reverse))))))

(fn ConstructionScript)